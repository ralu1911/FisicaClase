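; BP_Grenade is a grenade projectile that explodes when its Hit event fires.
; On hit it disables physics and collision, hides its sphere, stops movement and plays explosion particles and sound.
; It also spawns a short-lived FS_MasterField at the hit location with zero directional magnitude and triggers it, likely to break Chaos destructibles.
; The actor destroys itself once the explosion particle system finishes.
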(event `self.ReceiveBeginPlay`
  (add `ParticleSystemComponent.OnSystemFinished` (`self.ExplosionPS`) (delegate `Destroy`)))

(event `Destroy`
  (params (PSystem :type "ParticleSystemComponent Object Reference"))
  (`self.K2_DestroyActor`))

(event `self.ReceiveHit`
  (params (MyComp :type "PrimitiveComponent Object Reference") (Other :type "Actor Object Reference") (OtherComp :type "PrimitiveComponent Object Reference") (bSelfMoved :type Boolean) (HitLocation :type "Vector Structure") (HitNormal :type "Vector Structure") (NormalImpulse :type "Vector Structure") (Hit :type "HitResult Structure (by ref)"))
  (`PrimitiveComponent.SetSimulatePhysics` (`self.CollisionComp`) false)
  (`PrimitiveComponent.SetCollisionEnabled` (`self.CollisionComp`) "NoCollision")
  (`ActorComponent.Activate` (`self.ExplosionPS`) false)
  (`GameplayStatics.PlaySoundAtLocation` "/Game/StarterContent/Audio/Explosion01.Explosion01" (`self.K2_GetActorLocation`) (struct) 0.7 1.0 0.0 null null null null)
  (`SceneComponent.SetVisibility` (`self.Sphere`) false false)
  (`MovementComponent.StopMovementImmediately` (`self.ProjectileMovement`))
  (bind _returnvalue (`|SpawnActorFromClass` "/Game/FS_MasterField.FS_MasterField_C" (`KismetMathLibrary.Conv_VectorToTransform` HitLocation) "Undefined" "MultiplyWithRoot" null null))
  (set `/Game/FS_MasterField.ActivationType` "NewEnumerator4" _returnvalue)
  (`self.SetLifeSpan` _returnvalue 0.1)
  (set `/Game/FS_MasterField.DirectionalMagnitude` 0.0 _returnvalue)
  (`/Game/FS_MasterField.CE_Trigger` _returnvalue))

(fn `UserConstructionScript`)