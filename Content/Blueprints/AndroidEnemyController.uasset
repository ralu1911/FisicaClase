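; AI controller for an Android enemy that chases the player when perceived and otherwise patrols random points through a behavior tree.
; On possess it runs AndroidEnemyBT.
; AI Perception updates feed the blackboard, setting line of sight and the enemy actor when a Player-tagged actor is sensed.
; Otherwise a timer starts, clearing both keys after a delay, so losing sight has a grace period.
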(event `self.ReceivePossess`
  (params (PossessedPawn :type "Pawn Object Reference"))
  ;[1 1 1] Alternativa con IA (BTs y BB), aunque NO LO VAMOS A EXPLICAR TODAVÍA: Ejecuta una serie de tareas, de modo que cuando percibe al jugador, lo persigue... y si no, patrulla en puntos aleatorios
  (`self.RunBehaviorTree` "/Game/AI/AndroidEnemyBT.AndroidEnemyBT"))

(event `self.AIPerception.OnTargetPerceptionUpdated`
  (params (Actor :type "Actor Object Reference") (Stimulus :type "AIStimulus Structure"))
  (bind _blackboard (`self.Blackboard`))
  ;[1 1 1] Alternativa con IA (BTs y BB), aunque NO LO VAMOS A EXPLICAR TODAVÍA: Ejecuta una serie de tareas, de modo que cuando percibe al jugador, lo persigue... y si no, patrulla en puntos aleatorios
  (if (and (`self.ActorHasTag` Actor "Player") (`.bSuccessfullySensed` (break `AIStimulus` Stimulus)))
    (`KismetSystemLibrary.K2_ClearAndInvalidateTimerHandle` (`self.EnemyTimer`))
    (`BlackboardComponent.SetValueAsBool` _blackboard (`self.HasLineOfSight`) true)
    (`BlackboardComponent.SetValueAsObject` _blackboard (`self.EnemyActor`) Actor)
    (else
      (bind _returnvalue (`KismetSystemLibrary.K2_SetTimerDelegate` (delegate `StartEnemyTimer`) (`self.LineOfSightTimer`)))
      (set `self.EnemyTimer` _returnvalue))))

(event `StartEnemyTimer`
  (bind _blackboard (`self.Blackboard`))
  ;[1 1 1] Alternativa con IA (BTs y BB), aunque NO LO VAMOS A EXPLICAR TODAVÍA: Ejecuta una serie de tareas, de modo que cuando percibe al jugador, lo persigue... y si no, patrulla en puntos aleatorios
  (`BlackboardComponent.SetValueAsBool` _blackboard (`self.HasLineOfSight`) false)
  (`BlackboardComponent.SetValueAsObject` _blackboard (`self.EnemyActor`) null))

(fn `UserConstructionScript`)