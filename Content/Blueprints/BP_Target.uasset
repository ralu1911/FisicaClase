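; BP_Target is a destructible statue target that swaps from a static mesh to a Chaos Geometry Collection when hit hard enough.
; On a hit whose impulse exceeds the collection's first damage threshold, it hides the mesh, stops its physics, assigns the statue collection and damages itself by the impulse magnitude.
; Its damage handler prints that value and applies it as external strain at the stored hit location.
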(event `self.ReceiveHit`
  (params (MyComp :type "PrimitiveComponent Object Reference") (Other :type "Actor Object Reference") (OtherComp :type "PrimitiveComponent Object Reference") (bSelfMoved :type Boolean) (HitLocation :type "Vector Structure") (HitNormal :type "Vector Structure") (NormalImpulse :type "Vector Structure") (Hit :type "HitResult Structure (by ref)"))
  (bind _returnvalue (`KismetMathLibrary.VSize` NormalImpulse))
  (bind _staticmesh (`self.StaticMesh`))
  (set `self.Location` HitLocation)
  (if (> _returnvalue (`|GetArrayItem` (`GeometryCollectionComponent.DamageThreshold` (`self.GeometryCollection`))))
    (`SceneComponent.SetVisibility` _staticmesh false false)
    (`PrimitiveComponent.SetSimulatePhysics` _staticmesh false)
    (`GeometryCollectionComponent.SetRestCollection` (`self.GeometryCollection`) (`self.GC_Statue`) true)
    (`GameplayStatics.ApplyDamage` self _returnvalue null null "/Engine/EngineDamageTypes/DmgTypeBP_Environmental.DmgTypeBP_Environmental_C")))

(event `self.ReceiveBeginPlay`
  (add `Actor.OnTakeAnyDamage` (delegate `Damage`))
  (`GeometryCollectionComponent.SetEnableDamageFromCollision` (`self.GeometryCollection`) true))

(event `Damage`
  (params (DamagedActor :type "Actor Object Reference") (Damage :type "Float (single-precision)") (DamageType :type "DamageType Object Reference") (InstigatedBy :type "Controller Object Reference") (DamageCauser :type "Actor Object Reference"))
  (`KismetSystemLibrary.PrintString` (`KismetStringLibrary.Conv_DoubleToString` Damage))
  (`GeometryCollectionComponent.ApplyExternalStrain` (`self.GeometryCollection`) 0 (`self.Location`) 0.0 0 1.0 Damage))

(fn `UserConstructionScript`)